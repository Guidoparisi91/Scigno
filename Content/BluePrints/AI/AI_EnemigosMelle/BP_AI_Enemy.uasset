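; BP_AI_Enemy is the AI controller for melee enemies, running the BT_Enemigos behavior tree on possession.
; Its AI perception updates react only to BP_PersonajeHeroe, writing the hero to a blackboard key when sensed and clearing it when lost.
; Both outcomes print debug messages, and a disconnected branch that would pass the hero's transform never runs.
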(event OnTargetPerceptionUpdated(AIPerception)
  (params (Actor :type Actor%20Object%20Reference) (Stimulus :type AI%20Stimulus%20Structure))
  (bind _key_name (Variables|Default|GetKey%20Name))
  (bind _asbp_personaje_heroe (Utilities|Casting|CastToBP_PersonajeHeroe Actor))
  (if (.bsuccessfullysensed Stimulus)
    (AI|Components|Blackboard|SetValueasObject (AI|GetBlackboard 0) _key_name _asbp_personaje_heroe)
    (Development|PrintString "ve al objetivo")
    (else
      (AI|Components|Blackboard|SetValueasObject (AI|GetBlackboard 0) _key_name 0)
      (Development|PrintString "no ve al objetivo"))))

(event EventPossess
  (params (PossessedPawn :type Pawn%20Object%20Reference))
  (AI|RunBehaviorTree "/Game/BluePrints/AI/AI_EnemigosMelle/BT_Enemigos.BT_Enemigos"))

(fn ConstructionScript)