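; Health component that tracks current health and a death flag for its owner.
; DisminuirVida subtracts damage from VidaActual and broadcasts SeBajoVida with current and maximum health, capping only the broadcast value at a hardcoded 100 rather than VidaMaxima.
; At zero or below it sets EstaMuerto and prints a debug message, with no lower clamp on health.
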(event EventBeginPlay)

(event EventTick
  (params (DeltaSeconds :type Float%20%28single-precision%29)))

(fn DisminuirVida
  (params (daño :type Float%20%28double-precision%29))
  (bind _vidamaxima (Variables|vida|GetVidaMaxima))
  (bind _output_get (Variables|vida|SetVidaActual (- (Variables|vida|GetVidaActual) daño)))
  (if (> (Variables|vida|GetVidaActual) 1e+02)
    (Default|CallSeBajoVida 1e+02 _vidamaxima)
    (else
      (Default|CallSeBajoVida (Variables|vida|GetVidaActual) _vidamaxima)))
  (if (<= _output_get 0.0)
    (Variables|Default|SetestaMuerto true)
    (Development|PrintString "se murio!!!!!!!!!!!!!!")))