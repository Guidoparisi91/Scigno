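; Game instance Blueprint that manages the game's save slots.
; On Init it loads each slot named in NivelSlot, or creates and saves a new BP_SaveGame for missing ones, collecting them in SaveGames.
; SaveCurrentGame copies StructGameInstance into the active SaveGame, writes it to SlotName and prints a confirmation.
; LoadGame opens lvl_prueba_IA, selects the chosen SaveGames entry and sets the SaveLoad flag.
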(event EventInit
  (bind _savegames (Variables|Default|GetsaveGames))
  (for _array_element (Variables|Default|GetNivelSlot)
    (bind _returnvalue (SaveGame|DoesSaveGameExist _array_element))
    (if _returnvalue
      (bind _returnvalue_2 (SaveGame|LoadGamefromSlot _array_element))
      (bind _asbp_save_game (Utilities|Casting|CastToBP_SaveGame _returnvalue_2))
      (bind _output_get (Variables|Default|SetsaveGame _asbp_save_game))
      (bind _returnvalue_3 (Utilities|Array|AddUnique (Variables|Default|GetsaveGames) _output_get))
      (SaveGame|SaveGametoSlot 0 _array_element _returnvalue_3)
      (else
        (bind _returnvalue_4 (SaveGame|CreateSaveGameObject "/Game/BluePrints/Save/BP_SaveGame.BP_SaveGame_C"))
        (bind _output_get_2 (Variables|Default|SetsaveGame _returnvalue_4))
        (bind _returnvalue_5 (Utilities|Array|AddUnique _savegames _output_get_2))
        (Default|SetStruct (Utilities|Array|Get(acopy) _savegames _returnvalue_5) (Utilities|Struct|MakeS_StructureGame "0.000000,0.000000,0.000000|0.000000,0.000000,0.000000|1.000000,1.000000,1.000000" "0001.01.01-00.00.00" 0 0 0.0 0.0 0.0 0.0 true ""))
        (SaveGame|SaveGametoSlot (Utilities|Array|Get(acopy) _savegames _returnvalue_5) _array_element)))))

(fn SaveCurrentGame
  (params (struct :type S%20Structure%20Game%20Structure))
  (bind _slotname (Variables|Default|GetslotName))
  (Default|SetStruct (Variables|Default|GetsaveGame) (Variables|Default|GetstructGameInstance))
  (bind _returnvalue (SaveGame|SaveGametoSlot (Variables|Default|GetsaveGame) _slotname))
  (if _returnvalue
    (Development|PrintString (Utilities|String|Append "se guardo el slot :  
" _slotname) true true "(R=1.000000,G=0.538612,B=0.000000,A=1.000000)" 5.0)))

(fn LoadGame
  (params (slot :type Integer))
  (Game|OpenLevel(byName) "lvl_prueba_IA")
  (Variables|Default|SetsaveGame (Utilities|Array|Get(acopy) (Variables|Default|GetsaveGames) slot))
  (Variables|Default|SetsaveLoad? true))