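; BP_Viñetas_02 is a prop, apparently a comic-panel pickup or trigger, that unlocks the hero's melee weapon and clears a barricade.
; On overlap it runs the parent's overlap logic, then continues only if the other actor is BP_PersonajeHeroe.
; It sets the hero's melee unlock flag and destroys every Bp_espinas (thorns) actor tagged "barricada01", linking trigger to barricade by tag.
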(event EventBeginPlay
  (|CallParentFunction) ; This node is disabled and will not be called.\nDrag off pins to build functionality.
)

(event Collision|EventActorBeginOverlap
  (params (OtherActor :type Actor%20Object%20Reference))
  (|CallParentFunction OtherActor)
  (bind _asbp_personaje_heroe (Utilities|Casting|CastToBP_PersonajeHeroe OtherActor))
  (Variables|/Game/BluePrints/Character/BP_PersonajeHeroe.BP_PersonajeHeroe_C|SetArmaMeleeDesbloqueada _asbp_personaje_heroe true)
  (bind _outactors (Actor|GetAllActorsOfClasswithTag "/Game/BluePrints/Props/bp_espinas.bp_espinas_C" "barricada01"))
  (for _array_element _outactors
    (Actor|DestroyActor _array_element)))

(event EventTick
  (params (DeltaSeconds :type Float%20%28single-precision%29))
  (|CallParentFunction DeltaSeconds) ; This node is disabled and will not be called.\nDrag off pins to build functionality.
)

(fn ConstructionScript
  (|CallParentFunction))