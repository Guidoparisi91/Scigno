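; BP_Viñetas is a prop that triggers the showing and hiding of a vignette image as actors enter and leave its overlap.
; On begin and end overlap, it sends MuestraViñeta or OcultaViñeta with its Imagen variable to actors implementing BPI_Interacciones.
; The receiving actor handles the display, while the prop's own AgarraAlmas and MuestraViñeta functions are empty stubs.
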(event EventBeginPlay)

(event Collision|EventActorBeginOverlap
  (params (OtherActor :type Actor%20Object%20Reference))
  (if (Utilities|DoesObjectImplementInterface OtherActor "/Game/BluePrints/Interface/BPI_Interacciones.BPI_Interacciones_C")
    (Class|BPIInteracciones|MuestraViñeta(Message) OtherActor (Variables|Default|Getimagen))))

(event EventTick
  (params (DeltaSeconds :type Float%20%28single-precision%29)))

(event Collision|EventActorEndOverlap
  (params (OtherActor :type Actor%20Object%20Reference))
  (if (Utilities|DoesObjectImplementInterface OtherActor "/Game/BluePrints/Interface/BPI_Interacciones.BPI_Interacciones_C")
    (Class|BPIInteracciones|OcultaViñeta(Message) OtherActor (Variables|Default|Getimagen))))

(fn ConstructionScript)

(fn AgarraAlmas
  (return 0.0))

(fn MuestraViñeta
  (params (imagen :type Texture%202D%20Object%20Reference)))