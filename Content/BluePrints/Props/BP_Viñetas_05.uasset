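; BP_Viñetas_05 is a viñeta prop that unlocks the hero's ranged weapon on overlap.
; It runs the parent overlap logic, then casts the actor to BP_PersonajeHeroe and sets ArmaRangoDesbloqueada, printing a debug message if the cast fails.
; Unconnected nodes for refilling soul energy, updating values, hiding a key and revealing the "viñeta06" actor never run.
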(event EventBeginPlay
  (|CallParentFunction) ; This node is disabled and will not be called.\nDrag off pins to build functionality.
)

(event Collision|EventActorBeginOverlap
  (params (OtherActor :type Actor%20Object%20Reference))
  (|CallParentFunction OtherActor)
  (bind _asbp_personaje_heroe (Utilities|Casting|CastToBP_PersonajeHeroe OtherActor)
    (:then
      (Variables|/Game/BluePrints/Character/BP_PersonajeHeroe.BP_PersonajeHeroe_C|SetArmaRangoDesbloqueada _asbp_personaje_heroe true))
    (:CastFailed
      (Development|PrintString "fallo el casteo"))))

(event EventTick
  (params (DeltaSeconds :type Float%20%28single-precision%29))
  (|CallParentFunction DeltaSeconds) ; This node is disabled and will not be called.\nDrag off pins to build functionality.
)

(fn ConstructionScript
  (|CallParentFunction))