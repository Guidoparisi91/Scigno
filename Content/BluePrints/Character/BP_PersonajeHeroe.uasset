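; Player hero character with flipbook animation, Enhanced Input movement, an orthographic camera zoom-out at level start and a HUD.
; Movement direction orients the melee box, area-attack flipbook and projectile direction.
; Melee damages enemies overlapping the box, while area and ranged attacks spend soul energy gained through an interaction interface.
; The health component's delegate updates the HUD and, at zero, plays death, shows a confirmation screen and saves through the GameInstance.
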(event OnComponentBeginOverlap(Box)
  (params (OverlappedComponent :type Primitive%20Component%20Object%20Reference) (OtherActor :type Actor%20Object%20Reference) (OtherComp :type Primitive%20Component%20Object%20Reference) (OtherBodyIndex :type Integer) (bFromSweep :type Boolean) (SweepResult :type Hit%20Result%20Structure%20%28by%20ref%29))
  (bind _widgethub (Variables|Default|GetwidgetHub))
  (if (Utilities|DoesObjectImplementInterface OverlappedComponent "/Game/BluePrints/Interface/BPI_Interacciones.BPI_Interacciones_C")
    (bind _cantalmas (Class|BPIInteracciones|AgarraAlmas(Message) OverlappedComponent))
    (CallFunction|SumarEnergia _cantalmas)
    (UserInterface|Animation|PlayAnimation _widgethub (Variables|/Game/UX_UI/WidGets/WB_Hub.WB_Hub_C|Getviñeta _widgethub) 0.0 1 "Forward" 1.0 false)))

(event Custom|ActualizarVidaEnHub
  (params (VidaActual :type Float%20%28double-precision%29) (VidaMaxima :type Float%20%28double-precision%29))
  (Default|EventSetearVidaEvent (Variables|Default|GetwidgetHub) (/ VidaActual VidaMaxima) (Math|Float|Truncate VidaMaxima) (Math|Float|Truncate VidaActual))
  (if (<= (Variables|/Game/BluePrints/BPC_ComponenteSalud.BPC_ComponenteSalud_C|GetVidaActual (Variables|Default|GetBPC_ComponenteSalud)) 0.0)
    (if (not (Variables|Default|GetestaMuerto?))
      (|PlayAnimationOverridewithCallbacks (Class|PaperZDCharacter|GetAnimInstance) "/Game/Ani/CharacterHero/AnimSequences/AS_PersonajeHeroeMuere.AS_PersonajeHeroeMuere" "AS_Muere" 0.8 0.0
        (:then
          (Variables|Default|SetestaMuerto? true)
          (Pawn|Components|CharacterMovement|DisableMovement (Variables|Character|GetCharacterMovement))
          ;[1 1 1] ver que se hace cuando muere
          (CallFunction|MuestraPantallaConfirmacion))))))

(event Custom|camaraDeInicio
  ;[1 1 1] alejamiento de la camara al comenzar el nivel
  (Class|CameraComponent|SetOrthoWidth (Variables|Default|GetCamera) (Variables|Default|GetensancharPantalla))
  (Variables|Default|SetensancharPantalla (+ (Variables|Default|GetensancharPantalla) 5.0))
  (if (>= (Variables|Default|GetensancharPantalla) 2e+03)
    (Utilities|Time|ClearandInvalidateTimerbyHandle (stale EventBeginPlay _returnvalue))))

(event Input|EnhancedActionEvents|EnhancedInputActionIA_Movimiento
  (params (ActionValue :type Vector%202D%20Structure) (ElapsedSeconds :type Float%20%28double-precision%29) (TriggeredSeconds :type Float%20%28double-precision%29) (InputAction :type Input%20Action%20Object%20Reference :default "/Game/BluePrints/Character/Inputs/IA_Movimiento.IA_Movimiento"))
  ;[1 1 1] se mueve mientras no este atacando
  (if (not (Variables|Default|GetestaAtacando?))
    (Pawn|Input|AddMovementInput "1.000000,0.000000,0.000000" (.x ActionValue) false)
    (Pawn|Input|AddMovementInput "0.000000,1.000000,0.000000" (.y ActionValue) false)
    (CallFunction|SetDireccionDeColision)))

(event Input|EnhancedActionEvents|EnhancedInputActionIA_Ataque
  (params (ActionValue :type Boolean) (ElapsedSeconds :type Float%20%28double-precision%29) (TriggeredSeconds :type Float%20%28double-precision%29) (InputAction :type Input%20Action%20Object%20Reference :default "/Game/BluePrints/Character/Inputs/IA_Ataque.IA_Ataque"))
  ;[1 1 1] muestra la animacion de ataque
  (if (and (not (Variables|Default|GetestaAtacando?)) (not (Variables|Default|GetestaMuerto?)))
    (|PlayAnimationOverridewithCallbacks (Variables|/Script/PaperZD.PaperZDAnimationComponent|GetAnimInstance (Variables|Default|GetAnimationComponent)) "/Game/Ani/CharacterHero/AnimSequences/AS_PersonajeHeroeAttack.AS_PersonajeHeroeAttack" "Attack" 1.0 0.0
      (:then
        (Variables|Default|SetestaAtacando? true))
      (:OnCompleted
        (Variables|Default|SetestaAtacando? false :!label _label))
      (:OnCancelled
        (goto _label)))))

(event Input|EnhancedActionEvents|EnhancedInputActionIA_Salir
  (params (ActionValue :type Boolean) (ElapsedSeconds :type Float%20%28double-precision%29) (TriggeredSeconds :type Float%20%28double-precision%29) (InputAction :type Input%20Action%20Object%20Reference :default "/Game/BluePrints/Character/Inputs/IA_Salir.IA_Salir"))
  (Game|OpenLevel(byName) "Lvl_PantallaInicio"))

(event Input|EnhancedActionEvents|EnhancedInputActionIA_AtaqueRango
  (params (ActionValue :type Boolean) (ElapsedSeconds :type Float%20%28double-precision%29) (TriggeredSeconds :type Float%20%28double-precision%29) (InputAction :type Input%20Action%20Object%20Reference :default "/Game/BluePrints/Character/Inputs/IA_AtaqueRango.IA_AtaqueRango"))
  (bind _energiamaxima (Variables|Default|GetEnergiaMaxima))
  ;[1 1 1] DISPARA PROYECTIL
  (if (>= (Variables|Default|GetEnergiaAlmas) 1e+01)
    (bind _output_get (Variables|Default|SetEnergiaAlmas (- (Variables|Default|GetEnergiaAlmas) 1e+01)))
    (Game|SpawnActorfromClass "/Game/BluePrints/Character/BP_ProyectilHeroe.BP_ProyectilHeroe_C" (Math|Transform|MakeTransform (Transformation|GetActorLocation) "0, 0, 0" "1.000000,1.000000,1.000000") "AdjustIfPossibleButAlwaysSpawn" "MultiplyWithRoot" 0 (Variables|Default|GetdireccionProyectil) 1e+03 0)
    (Default|SetearEnergia (Variables|Default|GetwidgetHub) (/ _output_get _energiamaxima) (Math|Float|Truncate _output_get) (Math|Float|Truncate _energiamaxima))))

(event Input|EnhancedActionEvents|EnhancedInputActionIA_AtaqueArea
  (params (ActionValue :type Boolean) (ElapsedSeconds :type Float%20%28double-precision%29) (TriggeredSeconds :type Float%20%28double-precision%29) (InputAction :type Input%20Action%20Object%20Reference :default "/Game/BluePrints/Character/Inputs/IA_AtaqueArea.IA_AtaqueArea"))
  (bind _energiamaxima (Variables|Default|GetEnergiaMaxima))
  ;[1 1 1] Ataque de area
  (if (and (not (Variables|Default|GetestaAtacando?)) (>= (Variables|Default|GetEnergiaAlmas) 5.0))
    (Variables|Default|SetestaAtacando? true)
    (bind _output_get (Variables|Default|SetEnergiaAlmas (- (Variables|Default|GetEnergiaAlmas) 5.0)))
    (Sprite|SetSpriteColor (Variables|Default|GetFB_AtaqueArea) (Utilities|Struct|MakeLinearColor 1.0 1.0 1.0 0.5))
    (for _array_element (Collision|GetOverlappingActors (Variables|Default|GetFB_AtaqueArea) "/Game/BluePrints/Character/BP_PersonajeEnemigoBase.BP_PersonajeEnemigoBase_C" :!class /Script/Engine.PrimitiveComponent)
      (Game|Damage|ApplyDamage _array_element 5e+01 0 0)
      (Development|PrintString (Utilities|GetDisplayName _array_element)))
    (Default|SetearEnergia (Variables|Default|GetwidgetHub) (/ _output_get _energiamaxima) (Math|Float|Truncate _output_get) (Math|Float|Truncate _energiamaxima))
    (Utilities|FlowControl|Delay (Variables|Default|GetCoolDownTime))
    (Variables|Default|SetestaAtacando? false)
    (Sprite|SetSpriteColor (Variables|Default|GetFB_AtaqueArea) (Utilities|Struct|MakeLinearColor 1.0 1.0 1.0 0.0))))

(event EventBeginPlay
  (CallFunction|AddMapping)
  (CallFunction|CreateUi)
  (EventDispatchers|BindEventtoSeBajoVida (Variables|Default|GetBPC_ComponenteSalud) (delegate Custom|ActualizarVidaEnHub))
  ;[1 1 1] alejamiento de la camara al comenzar el nivel
  (bind _returnvalue (Utilities|Time|SetTimerbyEvent (delegate Custom|camaraDeInicio) 0.01 true true)))

(event EventAtaca
  ;[1 1 1] chequea ataque y se le pega a un enemigo le aplica daño
  (if (not (Variables|Default|GetestaMuerto?))
    (for _array_element (Collision|GetOverlappingActors (Variables|Collision|GetBox) "/Game/BluePrints/Character/BP_PersonajeEnemigoBase.BP_PersonajeEnemigoBase_C" :!class /Script/Engine.PrimitiveComponent)
      (Game|Damage|ApplyDamage _array_element 4e+01 0 0)
      (Development|PrintString (Utilities|String|Append "aplica daño a: " (Utilities|GetDisplayName _array_element))))))

(event EventTick
  (params (DeltaSeconds :type Float%20%28single-precision%29)))

(event EventMuestraPantallaConfirmacion
  ;[1 1 1] Pantalla confirmacion
  (Default|MostrarConfirmacion (Variables|Default|GetwidgetHub))
  (Variables|/Script/Engine.PlayerController|SetbShowMouseCursor (Game|GetPlayerController 0) true)
  (bind _asbp_ginstance (Utilities|Casting|CastToBP_GInstance (Game|GetGameInstance)))
  (bind _structactual (CallFunction|PasarStructDatos))
  (Default|SaveCurrentGame _asbp_ginstance _structactual))

(event EventOcultaPantallaConfirmacion
  ;[1 1 1] Pantalla confirmacion
  (Default|OcultarConfirmacion (Variables|Default|GetwidgetHub))
  (Variables|/Script/Engine.PlayerController|SetbShowMouseCursor (Game|GetPlayerController 0) false))

(event EventOcultaViñeta
  (params (imagen :type Texture%202D%20Object%20Reference))
  (bind _widgethub (Variables|Default|GetwidgetHub))
  ;[1 1 1] oculta viñeta
  (Appearance|SetBrushfromTexture (Variables|/Game/UX_UI/WidGets/WB_Hub.WB_Hub_C|GetImage_0 _widgethub) imagen false)
  (UserInterface|Animation|PlayAnimation _widgethub (Variables|/Game/UX_UI/WidGets/WB_Hub.WB_Hub_C|Getviñeta _widgethub) 0.0 1 "Reverse" 0.5 false))

(fn ConstructionScript
  (|CallParentFunction))

(fn AddMapping
  (bind _asplayer_controller (Utilities|Casting|CastToPlayerController (Pawn|GetController)))
  (Input|AddMappingContext (PlayerController|LocalPlayerSubsystems|GetEnhancedInputLocalPlayerSubsystem _asplayer_controller) "/Game/BluePrints/Character/Inputs/IM_Character.IM_Character" 0 "(bIgnoreAllPressedKeysUntilRelease=True,bForceImmediately=False,bNotifyUserSettings=False)"))

(fn CreateUi
  (bind _returnvalue (UserInterface|CreateWidget "/Game/UX_UI/WidGets/WB_Hub.WB_Hub_C"))
  (UserInterface|Viewport|AddtoViewport _returnvalue 0)
  (Variables|Default|SetwidgetHub _returnvalue))

(fn SetDireccionDeColision
  (bind _returnvalue (Transformation|GetVelocity))
  (bind _returnvalue_2 (Transformation|GetActorLocation))
  (bind _box (Variables|Collision|GetBox))
  (bind _returnvalue_3 (Class|KismetMathLibrary|VectorNormal2D _returnvalue 0.0001))
  (bind _returnvalue_4 (Math|Conversions|RotationFromXVector _returnvalue))
  ;[1 1 1] coloca la caja y el triangulo de colision en direccion donde esta mirando
  (if (> (Math|Vector|VectorLength _returnvalue) 0.0)
    (Transformation|SetWorldLocation _box (Math|Vector|MakeVector (+ (.x _returnvalue_2) (* 5e+01 (.x _returnvalue_3))) (+ (.y _returnvalue_2) (* 5e+01 (.y _returnvalue_3))) 3e+01) false false)
    (Transformation|SetWorldRotation _box (Math|Rotator|MakeRotator 0.0 0.0 (.yaw _returnvalue_4)) false false)
    (Variables|Default|SetdireccionProyectil (Math|Vector|MakeVector (.x _returnvalue_3) (.y _returnvalue_3) 0.0))
    (Transformation|SetRelativeRotation (Variables|Default|GetFB_AtaqueArea) (Math|Rotator|MakeRotator 9e+01 (.pitch _returnvalue_4) (+ (.yaw _returnvalue_4) -9e+01)) false false)))

(fn SumarEnergia
  (params (cantidadEnergia :type Float%20%28double-precision%29))
  (Variables|Default|SetEnergiaAlmas (Math|Float|Clamp(Float) (+ cantidadEnergia (Variables|Default|GetEnergiaAlmas)) 0.0 (Variables|Default|GetEnergiaMaxima))))

(fn SumarExperiencia
  (params (experiencia :type Integer))
  (Variables|Default|SetExperiencia (+ experiencia (Variables|Default|GetExperiencia))))

(fn AceptaAlmas
  (params (cantAlmas :type Float%20%28double-precision%29))
  (bind _energiaalmas (Variables|Default|GetEnergiaAlmas))
  (bind _energiamaxima (Variables|Default|GetEnergiaMaxima))
  (CallFunction|SumarEnergia cantAlmas)
  (Default|SetearEnergia (Variables|Default|GetwidgetHub) (/ _energiaalmas _energiamaxima) (Math|Float|Truncate _energiaalmas) (Math|Float|Truncate _energiamaxima))
  (return))

(fn AgarraAlmas
  (return 0.0))

(fn MuestraViñeta
  (params (imagen :type Texture%202D%20Object%20Reference))
  (bind _widgethub (Variables|Default|GetwidgetHub))
  (Appearance|SetBrushfromTexture (Variables|/Game/UX_UI/WidGets/WB_Hub.WB_Hub_C|GetImage_0 _widgethub) imagen false)
  (UserInterface|Animation|PlayAnimation _widgethub (Variables|/Game/UX_UI/WidGets/WB_Hub.WB_Hub_C|Getviñeta _widgethub) 0.0 1 "Forward" 1.0 false)
  (return))

(fn PasarStructDatos
  (bind _bpc_componentesalud (Variables|Default|GetBPC_ComponenteSalud))
  (bind _returnvalue (Game|GetCurrentLevelName true))
  (return (Utilities|Struct|MakeS_StructureGame (Transformation|GetActorTransform) (Math|DateTime|Now) 0 (Variables|Default|GetExperiencia) (Variables|/Game/BluePrints/BPC_ComponenteSalud.BPC_ComponenteSalud_C|GetVidaActual _bpc_componentesalud) (Variables|/Game/BluePrints/BPC_ComponenteSalud.BPC_ComponenteSalud_C|GetVidaMaxima _bpc_componentesalud) (Variables|Default|GetEnergiaAlmas) (Variables|Default|GetEnergiaMaxima) true _returnvalue)))