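; Base character Blueprint with a sprite that handles taking damage, giving visual hit feedback.
; Any damage is passed to the health component (BPCComponenteSalud) to reduce life, and spawns a particle system at the actor's location.
; A looping timer then tints the sprite red and steps green and blue back up toward white, clearing itself and resetting once the fade completes.
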(event Custom|cambiaColor
  (Sprite|SetSpriteColor (Variables|Default|GetSprite) (Math|Color|MakeColor 1.0 (Variables|Default|GettiempoCambioColor) (Variables|Default|GettiempoCambioColor)))
  (bind _output_get (Variables|Default|SettiempoCambioColor (+ (Variables|Default|GettiempoCambioColor) 0.1)))
  (if (>= _output_get 1.0)
    (Utilities|Time|ClearandInvalidateTimerbyHandle (stale Game|Damage|EventAnyDamage _returnvalue))
    (Variables|Default|SettiempoCambioColor 0.0)))

(event Game|Damage|EventAnyDamage
  (params (Damage :type Float%20%28single-precision%29) (DamageType :type Damage%20Type%20Object%20Reference) (InstigatedBy :type Controller%20Object%20Reference) (DamageCauser :type Actor%20Object%20Reference))
  (Default|DisminuirVida (Variables|Default|GetBPC_ComponenteSalud) Damage)
  (Niagara|SpawnSystematLocation (Variables|Default|GetSystem%20Template) (Transformation|GetActorLocation))
  (bind _returnvalue (Utilities|Time|SetTimerbyEvent (delegate Custom|cambiaColor) 0.04 true)))

(fn ConstructionScript)