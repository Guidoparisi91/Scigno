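; Melee boss enemy character Blueprint that implements a close-range attack against the hero.
; The Ataca event stops movement and, if the boss is alive and neither attacking nor being hit, plays a PaperZD attack animation override while flagging EstaAtacando.
; When the animation completes, heroes overlapping the Box take damage and are pushed away through Mover; a cancelled animation only clears the attacking flag.
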(event EventBeginPlay
  (|CallParentFunction) ; This node is disabled and will not be called.\nDrag off pins to build functionality.
)

(event Collision|EventActorBeginOverlap
  (params (OtherActor :type Actor%20Object%20Reference))
  (|CallParentFunction OtherActor) ; This node is disabled and will not be called.\nDrag off pins to build functionality.
)

(event EventTick
  (params (DeltaSeconds :type Float%20%28single-precision%29))
  (|CallParentFunction DeltaSeconds) ; This node is disabled and will not be called.\nDrag off pins to build functionality.
)

(event EventAtaca
  ;[1 1 1] muestra la animacion de ataque
  (Components|Movement|StopMovementImmediately (Variables|Character|GetCharacterMovement))
  (if (Math|Boolean|ANDBoolean (Variables|Default|GetestaVivo?) (not (Variables|Default|GetestaAtacando?)) (not (Variables|Default|GetesAtacado?)))
    (|PlayAnimationOverridewithCallbacks (Variables|/Script/PaperZD.PaperZDAnimationComponent|GetAnimInstance (Variables|Default|GetAnimationComponent)) "/Game/Ani/CharacterEnemyBaseMeele/AnimSequences/AS_enemigoAttack.AS_enemigoAttack" "AttackEnemigoMeele" 1.0 0.0
      (:then
        (Variables|Default|SetestaAtacando? true))
      (:OnCompleted
        (Variables|Default|SetestaAtacando? false)
        (for _array_element (Collision|GetOverlappingActors (Variables|Default|GetBox) "/Game/BluePrints/Character/BP_PersonajeHeroe.BP_PersonajeHeroe_C" :!class /Script/Engine.PrimitiveComponent)
          (Game|Damage|ApplyDamage _array_element 5.0 0 0)
          (bind _asbp_personaje_heroe (Utilities|Casting|CastToBP_PersonajeHeroe _array_element))
          (Default|Mover _asbp_personaje_heroe (Math|Vector|Normalize (- (Transformation|GetActorLocation _array_element) (Transformation|GetActorLocation))))))
      (:OnCancelled
        (Variables|Default|SetestaAtacando? false)))))

(fn ConstructionScript
  (|CallParentFunction))