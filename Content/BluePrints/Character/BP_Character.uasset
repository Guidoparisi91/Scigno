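; Player character Blueprint that handles eight-direction movement on an isometric grid.
; On BeginPlay it adds the IM_Character Enhanced Input mapping context to its player controller.
; IA_Movimiento runs a nested branch chain on the input's X/Y signs, feeding fixed world directions to AddMovementInput.
; The mapping rotates input 45 degrees: diagonal input follows world axes, and straight input moves along world diagonals.
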(event Input|EnhancedActionEvents|EnhancedInputActionIA_Movimiento
  (params (ActionValue :type Vector%202D%20Structure) (ElapsedSeconds :type Float%20%28double-precision%29) (TriggeredSeconds :type Float%20%28double-precision%29) (InputAction :type Input%20Action%20Object%20Reference :default "/Game/BluePrints/Character/Inputs/IA_Movimiento.IA_Movimiento"))
  ;[1 1 1] Movimiento en la grilla isometrica
  (:Triggered
    (if (and (> (.x ActionValue) 0.0) (> (.y ActionValue) 0.0))
      (Pawn|Input|AddMovementInput (Math|Vector|MakeVector 1.0 0.0 0.0) 1.0 false)
      (elif (and (< (.x ActionValue) 0.0) (< (.y ActionValue) 0.0))
        (Pawn|Input|AddMovementInput (Math|Vector|MakeVector -1.0 0.0 0.0) 1.0 false)
        (elif (and (< (.x ActionValue) 0.0) (> (.y ActionValue) 0.0))
          (Pawn|Input|AddMovementInput (Math|Vector|MakeVector 0.0 1.0 0.0) 1.0 false)
          (elif (and (< (.y ActionValue) 0.0) (> (.x ActionValue) 0.0))
            (Pawn|Input|AddMovementInput (Math|Vector|MakeVector 0.0 -1.0 0.0) 1.0 false)
            (elif (and (< (.x ActionValue) 0.0) (== (.y ActionValue) 0.0))
              (Pawn|Input|AddMovementInput (Math|Vector|MakeVector -1.0 1.0 0.0) 1.0 false)
              (elif (and (> (.x ActionValue) 0.0) (== 0.0 (.y ActionValue)))
                (Pawn|Input|AddMovementInput (Math|Vector|MakeVector 1.0 -1.0 0.0) 1.0 false)
                (elif (and (< (.y ActionValue) 0.0) (== 0.0 (.x ActionValue)))
                  (Pawn|Input|AddMovementInput (Math|Vector|MakeVector -1.0 -1.0 0.0) 1.0 false)
                  (elif (and (> (.y ActionValue) 0.0) (== (.x ActionValue) 0.0))
                    (Pawn|Input|AddMovementInput (Math|Vector|MakeVector 1.0 1.0 0.0) 1.0 false)))))))))))

(event EventBeginPlay
  ;[1 1 1] Conectar inputs al character
  (bind _asplayer_controller (Utilities|Casting|CastToPlayerController (Pawn|GetController)))
  (Input|AddMappingContext (PlayerController|LocalPlayerSubsystems|GetEnhancedInputLocalPlayerSubsystem _asplayer_controller) "/Game/BluePrints/Character/Inputs/IM_Character.IM_Character" 0 "(bIgnoreAllPressedKeysUntilRelease=True,bForceImmediately=False,bNotifyUserSettings=False)"))

(event Collision|EventActorBeginOverlap
  (params (OtherActor :type Actor%20Object%20Reference)))

(event EventTick
  (params (DeltaSeconds :type Float%20%28single-precision%29)))

(fn ConstructionScript)