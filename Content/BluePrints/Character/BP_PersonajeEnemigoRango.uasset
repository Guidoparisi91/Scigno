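; Ranged enemy character that fires projectiles at the hero and drops a soul when killed.
; Ataca starts a looping timer at a random interval that halts movement, plays the shoot animation and spawns a projectile aimed at the hero, stopping once the hero is out of range.
; Health changes update the widget bar; at zero health it spawns BP_Almas and fades the sprite by timer before destroying itself.
; The death animation node is unconnected.
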(event SeBajoVida(BPC_ComponenteSalud)
  (params (VidaActual :type Float%20%28double-precision%29) (VidaMaxima :type Float%20%28double-precision%29))
  (bind _returnvalue (Transformation|GetActorLocation))
  ;[1 0.3719 0.3719] Se aplica daño, se anima la muerte, se destruye actor
  (bind _aswb_enemigo (Utilities|Casting|CastToWB_Enemigo (UserInterface|GetWidget (Variables|Default|GetWidget))))
  (Default|SetearVida _aswb_enemigo (/ VidaActual VidaMaxima))
  (if (<= VidaActual 0.0)
    (Variables|Default|SetestaVivo? false)
    (bind _returnvalue_2 (Utilities|Time|SetTimerbyEvent (delegate Custom|desvanecer%20enemigo) 0.011 true))
    (if (not (Variables|Default|GetestaVivo?))
      (Game|SpawnActorfromClass "/Game/BluePrints/Props/BP_Almas.BP_Almas_C" (Math|Transform|MakeTransform (Math|Vector|MakeVector (+ (.x _returnvalue) 0.0) (+ (.y _returnvalue) 0.0) 2e+02) "0, 0, 0" "1.000000,1.000000,1.000000") "AlwaysSpawn" "MultiplyWithRoot" 0 1e+01 (Math|Vector|Normalize (Transformation|GetActorLocation (Variables|Default|GetrefHeroe))) 0))))

(event Custom|disparaConstantemente
  (bind _returnvalue (Transformation|GetActorLocation))
  (bind _refheroe (Variables|Default|GetrefHeroe))
  (bind _returnvalue_2 (Transformation|GetActorLocation _refheroe))
  (bind _returnvalue_3 (- _returnvalue_2 _returnvalue))
  (bind _returnvalue_4 (Math|Vector|VectorLength _returnvalue_3))
  ;[1 1 1] Dispara hasta constantemente hasta que salga del radio
  (Components|Movement|StopMovementImmediately (Variables|Character|GetCharacterMovement))
  (if (Math|Boolean|ANDBoolean (Variables|Default|GetestaVivo?) true true)
    (|PlayAnimationOverridewithCallbacks (Variables|/Script/PaperZD.PaperZDAnimationComponent|GetAnimInstance (Variables|Default|GetAnimationComponent)) "/Game/Ani/CharacterEnemyRango/AnimSequences/AS_EnemigoRangoDispara.AS_EnemigoRangoDispara" "disparaRango" 1.0 0.0
      (:then
        (Game|SpawnActorfromClass "/Game/BluePrints/Character/BP_ProyectilEnemigo.BP_ProyectilEnemigo_C" (Math|Transform|MakeTransform _returnvalue "0, 0, 0" "1.000000,1.000000,1.000000") "AlwaysSpawn" "MultiplyWithRoot" 0 (Class|KismetMathLibrary|VectorNormal2D _returnvalue_3 0.0001) 7.5e+02 0)
        (if (> _returnvalue_4 1e+03)
          (Utilities|Time|ClearandInvalidateTimerbyHandle (stale EventAtaca _returnvalue))
          (else
            (Development|PrintString (Utilities|String|ToString(Float) _returnvalue_4))))))))

(event Custom|desvanecer%20enemigo
  ;[1 0.3719 0.3719] Se aplica daño, se anima la muerte, se destruye actor
  (Sprite|SetSpriteColor (Variables|Default|GetSprite) (Utilities|Struct|MakeLinearColor 1.0 1.0 1.0 (Variables|Default|Getalpha)))
  (bind _output_get (Variables|Default|Setalpha (- (Variables|Default|Getalpha) 0.01)))
  (if (<= _output_get 0.0)
    (Utilities|Time|ClearandInvalidateTimerbyHandle (stale SeBajoVida(BPC_ComponenteSalud) _returnvalue_2))
    (Actor|DestroyActor)))

(event EventBeginPlay
  (bind _outactors (Actor|GetAllActorsOfClass "/Game/BluePrints/Character/BP_PersonajeHeroe.BP_PersonajeHeroe_C"))
  (Variables|Default|SetrefHeroe (Utilities|Array|Get(acopy) _outactors)))

(event Collision|EventActorBeginOverlap
  (params (OtherActor :type Actor%20Object%20Reference)))

(event EventTick
  (params (DeltaSeconds :type Float%20%28single-precision%29)))

(event EventAtaca
  ;[1 1 1] Dispara hasta constantemente hasta que salga del radio
  (bind _returnvalue (Utilities|Time|SetTimerbyEvent (delegate Custom|disparaConstantemente) (Math|Random|RandomFloatinRange 1.5 2.5) true)))

(fn ConstructionScript
  (|CallParentFunction))

(fn AgarraAlmas
  (return 0.0))

(fn PasarStructDatos
  (return ""))

(fn PasarUbicacionHeroe
  (params (ubicacionHeroe :type Vector :default "0, 0, 0"))
  (Variables|Default|SetubicacionHeroe ubicacionHeroe)
  (return))

(fn RecibirUbicacionHeroe
  (return "0, 0, 0"))