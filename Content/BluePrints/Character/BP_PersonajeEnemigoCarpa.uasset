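; BP_PersonajeEnemigoCarpa is a sprite-animated enemy whose health and scale grow with its level, shown on a widget.
; The health component's damage event updates that widget and plays a hit or death animation override.
; Death starts a looping timer that fades the sprite until destruction.
; It also spawns souls, grants the hero experience and randomly drops a BP_Vida pickup.
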(event SeBajoVida(BPC_ComponenteSalud)
  (params (VidaActual :type Float%20%28double-precision%29) (VidaMaxima :type Float%20%28double-precision%29))
  (bind _returnvalue (Transformation|GetActorLocation))
  (bind _returnvalue_2 (Transformation|GetActorLocation))
  (bind _refheroe (Variables|Default|GetrefHeroe))
  (bind _returnvalue_3 (Transformation|GetActorLocation _refheroe))
  (bind _returnvalue_4 (Math|Vector|Normalize _returnvalue_3))
  ;[1 0.3719 0.3719] Se aplica daño, se anima la muerte, se destruye actor
  (bind _aswb_enemigo (Utilities|Casting|CastToWB_Enemigo (UserInterface|GetWidget (Variables|Default|GetWidget))))
  (Default|SetearVida _aswb_enemigo (/ VidaActual VidaMaxima))
  (if (<= VidaActual 0.0)
    (Variables|Default|SetestaVivo? (Variables|Default|GetEstaVivo?))
    (|PlayAnimationOverridewithCallbacks (Variables|/Script/PaperZD.PaperZDAnimationComponent|GetAnimInstance (Variables|Default|GetAnimationComponent)) "/Game/Ani/CharacterEnemyBaseMeele/AnimSequences/AS_EnemigoMuere.AS_EnemigoMuere" "EnemigoMuere" 0.5 0.0
      (:then
        (bind _returnvalue_5 (Utilities|Time|SetTimerbyEvent (delegate Custom|desvanecer%20enemigo) 0.011 true))
        (if (not (Variables|Default|GetestaVivo?))
          (Game|SpawnActorfromClass "/Game/BluePrints/Props/BP_Almas.BP_Almas_C" (Math|Transform|MakeTransform (Math|Vector|MakeVector (+ (.x _returnvalue) 0.0) (+ (.y _returnvalue) 0.0) 2e+02) "0, 0, 0" "1.000000,1.000000,1.000000") "AlwaysSpawn" "MultiplyWithRoot" 0 1e+01 _returnvalue_4 0)
          (Default|RecibeExperiencia (Variables|Default|GetrefHeroe) 10)
          (if (== (Math|Random|RandomIntegerinRange 1 5) 3)
            (Game|SpawnActorfromClass "/Game/BluePrints/Props/BP_Vida.BP_Vida_C" (Math|Transform|MakeTransform (Math|Vector|MakeVector (.x _returnvalue_2) (.y _returnvalue_2) 3e+02) "0, 0, 0" "1.000000,1.000000,1.000000") "AlwaysSpawn" "MultiplyWithRoot" 0 _returnvalue_4 0)))))
    (elif (not (Variables|Default|GetesAtacado?))
      (|PlayAnimationOverridewithCallbacks (Variables|/Script/PaperZD.PaperZDAnimationComponent|GetAnimInstance (Variables|Default|GetAnimationComponent)) "/Game/Ani/CharacterEnemyBaseMeele/AnimSequences/AS_EnemigoGotHit.AS_EnemigoGotHit" "EnemigoGotHit" 1.0 0.0
        (:then
          (Variables|Default|SetesAtacado? (Variables|Default|GetEsAtacado?)))
        (:OnCompleted
          (Variables|Default|SetesAtacado? (Variables|Default|GetEsAtacado?_0)))))))

(event Custom|desvanecer%20enemigo
  ;[1 0.3719 0.3719] Se aplica daño, se anima la muerte, se destruye actor
  (Sprite|SetSpriteColor (Variables|Default|GetSprite) (Utilities|Struct|MakeLinearColor 1.0 1.0 1.0 (Variables|Default|Getalpha)))
  (bind _output_get (Variables|Default|Setalpha (- (Variables|Default|Getalpha) 0.01)))
  (if (<= _output_get 0.0)
    (Utilities|Time|ClearandInvalidateTimerbyHandle (stale SeBajoVida(BPC_ComponenteSalud) _returnvalue_5))
    (Actor|DestroyActor)))

(event EventBeginPlay
  (bind _bpc_componentesalud (Variables|Default|GetBPC_ComponenteSalud))
  (bind _nivel (Variables|Default|GetNivel))
  (|CallParentFunction)
  (Variables|/Game/BluePrints/BPC_ComponenteSalud.BPC_ComponenteSalud_C|SetVidaActual _bpc_componentesalud (+ (* (Variables|Default|GetNivel) 10) (Variables|/Game/BluePrints/BPC_ComponenteSalud.BPC_ComponenteSalud_C|GetVidaActual _bpc_componentesalud)))
  (Variables|/Game/BluePrints/BPC_ComponenteSalud.BPC_ComponenteSalud_C|SetVidaMaxima _bpc_componentesalud (+ (* (Variables|Default|GetNivel) 10) (Variables|/Game/BluePrints/BPC_ComponenteSalud.BPC_ComponenteSalud_C|GetVidaActual _bpc_componentesalud)))
  (bind _aswb_enemigo (Utilities|Casting|CastToWB_Enemigo (UserInterface|GetWidget (Variables|Default|GetWidget))))
  (Default|MostrarNivel _aswb_enemigo _nivel)
  (Transformation|SetRelativeScale3D (Variables|Default|GetSprite) (Math|Conversions|ToVector(Float) (+ 1.0 (/ (Math|Conversions|ToFloat(Integer) _nivel) 1e+01)))))

(event Collision|EventActorBeginOverlap
  (params (OtherActor :type Actor%20Object%20Reference))
  (|CallParentFunction OtherActor) ; This node is disabled and will not be called.\nDrag off pins to build functionality.
)

(event EventTick
  (params (DeltaSeconds :type Float%20%28single-precision%29))
  (|CallParentFunction DeltaSeconds) ; This node is disabled and will not be called.\nDrag off pins to build functionality.
)

(fn ConstructionScript
  (|CallParentFunction))