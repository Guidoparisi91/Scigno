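; BP_ProyectilHeroe is the hero's projectile, which damages enemies and lives for two seconds.
; Each tick it moves by a local, unswept offset from DireccionProyectil and Velocidad, and orients FBProyectilBase using DireccionRotation's yaw, with roll switched by the direction's X value.
; A Sphere overlap with a BP_PersonajeEnemigoBase applies Daño and destroys the projectile, while other actors are ignored.
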(event OnComponentBeginOverlap(Sphere)
  (params (OverlappedComponent :type Primitive%20Component%20Object%20Reference) (OtherActor :type Actor%20Object%20Reference) (OtherComp :type Primitive%20Component%20Object%20Reference) (OtherBodyIndex :type Integer) (bFromSweep :type Boolean) (SweepResult :type Hit%20Result%20Structure%20%28by%20ref%29))
  (bind _asbp_personaje_enemigo_base (Utilities|Casting|CastToBP_PersonajeEnemigoBase OtherActor))
  (Game|Damage|ApplyDamage _asbp_personaje_enemigo_base (Variables|Default|Getdaño) 0 0)
  (Actor|DestroyActor))

(event EventBeginPlay
  (Actor|SetLifeSpan 2.0))

(event EventTick
  (params (DeltaSeconds :type Float%20%28single-precision%29))
  (bind _direccionproyectil (Variables|Default|GetdireccionProyectil))
  (bind _direccionrotation (Variables|Default|GetdireccionRotation))
  (bind _fb_proyectilbase (Variables|Default|GetFB_ProyectilBase))
  ;[1 1 1] para que se acomode el proyectil
  (Transformation|AddActorLocalOffset (* _direccionproyectil (Variables|Default|Getvelocidad) DeltaSeconds) false false)
  (if (<= (.X (Math|Vector|BreakVector _direccionproyectil)) 5.0)
    (Transformation|SetRelativeRotation _fb_proyectilbase (Math|Rotator|MakeRotator 9e+01 0.0 (.yaw _direccionrotation)) false false)
    (else
      (Transformation|SetRelativeRotation _fb_proyectilbase (Math|Rotator|MakeRotator 0.0 0.0 (.yaw _direccionrotation)) false false))))

(fn ConstructionScript)