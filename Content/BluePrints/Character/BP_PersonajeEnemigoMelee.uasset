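; Melee enemy character with an animated sprite whose health, damage, size and red tint can scale with its level.
; Each tick a hit box follows its movement direction; Ataca plays an attack animation, then damages overlapping heroes on completion.
; Health component changes update the overhead widget and play hit or death animations.
; Death spawns souls, sometimes a health pickup, grants the hero experience and fades the sprite before destroying the actor.
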(event SeBajoVida(BPC_ComponenteSalud)
  (params (VidaActual :type Float%20%28double-precision%29) (VidaMaxima :type Float%20%28double-precision%29))
  (bind _returnvalue (Transformation|GetActorLocation))
  (bind _returnvalue_2 (Transformation|GetActorLocation))
  (bind _refheroe (Variables|Default|GetrefHeroe))
  (bind _returnvalue_3 (Transformation|GetActorLocation _refheroe))
  (bind _returnvalue_4 (Math|Vector|Normalize _returnvalue_3))
  ;[1 0.3719 0.3719] Se aplica daño, se anima la muerte, se destruye actor
  (bind _aswb_enemigo (Utilities|Casting|CastToWB_Enemigo (UserInterface|GetWidget (Variables|Default|GetWidget))))
  (Default|SetearVida _aswb_enemigo (/ VidaActual VidaMaxima))
  (if (<= VidaActual 0.0)
    (Variables|Default|SetestaVivo? false)
    (|PlayAnimationOverridewithCallbacks (Variables|/Script/PaperZD.PaperZDAnimationComponent|GetAnimInstance (Variables|Default|GetAnimationComponent)) "/Game/Ani/CharacterEnemyBaseMeele/AnimSequences/AS_EnemigoMuere.AS_EnemigoMuere" "EnemigoMuere" 0.5 0.0
      (:then
        (bind _returnvalue_5 (Utilities|Time|SetTimerbyEvent (delegate Custom|desvanecer%20enemigo) 0.011 true))
        (if (not (Variables|Default|GetestaVivo?))
          (Game|SpawnActorfromClass "/Game/BluePrints/Props/BP_Almas.BP_Almas_C" (Math|Transform|MakeTransform (Math|Vector|MakeVector (+ (.x _returnvalue) 0.0) (+ (.y _returnvalue) 0.0) 2e+02) "0, 0, 0" "1.000000,1.000000,1.000000") "AlwaysSpawn" "MultiplyWithRoot" 0 1e+01 _returnvalue_4 0)
          (Default|RecibeExperiencia (Variables|Default|GetrefHeroe) 3)
          (if (== (Math|Random|RandomIntegerinRange 1 5) 3)
            (Game|SpawnActorfromClass "/Game/BluePrints/Props/BP_Vida.BP_Vida_C" (Math|Transform|MakeTransform (Math|Vector|MakeVector (.x _returnvalue_2) (.y _returnvalue_2) 3e+02) "0, 0, 0" "1.000000,1.000000,1.000000") "AlwaysSpawn" "MultiplyWithRoot" 0 _returnvalue_4 0)))))
    (elif (not (Variables|Default|GetesAtacado?))
      (|PlayAnimationOverridewithCallbacks (Variables|/Script/PaperZD.PaperZDAnimationComponent|GetAnimInstance (Variables|Default|GetAnimationComponent)) "/Game/Ani/CharacterEnemyBaseMeele/AnimSequences/AS_EnemigoGotHit.AS_EnemigoGotHit" "EnemigoGotHit" 1.0 0.0
        (:then
          (Variables|Default|SetesAtacado? true))
        (:OnCompleted
          (Variables|Default|SetesAtacado? false))))))

(event Custom|desvanecer%20enemigo
  ;[1 0.3719 0.3719] Se aplica daño, se anima la muerte, se destruye actor
  (Sprite|SetSpriteColor (Variables|Default|GetSprite) (Utilities|Struct|MakeLinearColor 1.0 1.0 1.0 (Variables|Default|Getalpha)))
  (bind _output_get (Variables|Default|Setalpha (- (Variables|Default|Getalpha) 0.01)))
  (if (<= _output_get 0.0)
    (Utilities|Time|ClearandInvalidateTimerbyHandle (stale SeBajoVida(BPC_ComponenteSalud) _returnvalue_5))
    (Actor|DestroyActor)))

(event EventBeginPlay
  (bind _bpc_componentesalud (Variables|Default|GetBPC_ComponenteSalud))
  (bind _sprite (Variables|Default|GetSprite))
  (bind _vidainicial (Variables|Default|GetVidaInicial))
  (bind _nivel (Variables|Default|Getnivel))
  (bind _returnvalue (Math|Conversions|ToFloat(Integer) _nivel))
  (bind _returnvalue_2 (/ _returnvalue 1e+01))
  (bind _returnvalue_3 (- 1.0 _returnvalue_2))
  (Utilities|FlowControl|Delay 0.2)
  (bind _outactors (Actor|GetAllActorsOfClass "/Game/BluePrints/Character/BP_PersonajeHeroe.BP_PersonajeHeroe_C"))
  (Variables|Default|SetrefHeroe (Utilities|Array|Get(acopy) _outactors))
  (Variables|/Game/BluePrints/BPC_ComponenteSalud.BPC_ComponenteSalud_C|SetVidaActual _bpc_componentesalud (+ (* (Variables|Default|Getnivel) 10) (Variables|/Game/BluePrints/BPC_ComponenteSalud.BPC_ComponenteSalud_C|GetVidaActual _bpc_componentesalud)))
  (if (!= _vidainicial 1e+02)
    (bind _output_get (Variables|/Game/BluePrints/BPC_ComponenteSalud.BPC_ComponenteSalud_C|SetVidaActual _bpc_componentesalud _vidainicial))
    (bind _output_get_2 (Variables|/Game/BluePrints/BPC_ComponenteSalud.BPC_ComponenteSalud_C|SetVidaMaxima _bpc_componentesalud (+ (* (Variables|Default|Getnivel) 10) (Variables|/Game/BluePrints/BPC_ComponenteSalud.BPC_ComponenteSalud_C|GetVidaActual _bpc_componentesalud))))
    (bind _aswb_enemigo (Utilities|Casting|CastToWB_Enemigo (UserInterface|GetWidget (Variables|Default|GetWidget))))
    (Default|SetearVida _aswb_enemigo 1.0)
    (Default|MostrarNivel _aswb_enemigo _nivel)
    (Transformation|SetRelativeScale3D _sprite (Math|Conversions|ToVector(Float) (+ 1.0 _returnvalue_2)))
    (Sprite|SetSpriteColor _sprite (Math|Color|MakeColor 1.0 _returnvalue_3 _returnvalue_3))))

(event EventTick
  (params (DeltaSeconds :type Float%20%28single-precision%29))
  (CallFunction|SetDireccionDeColision))

(event EventAtaca
  (bind _returnvalue (Math|Random|RandomFloatinRange 0.8 1.2))
  (bind _box (Variables|Default|GetBox))
  (bind _overlappingactors (Collision|GetOverlappingActors _box "/Game/BluePrints/Character/BP_PersonajeHeroe.BP_PersonajeHeroe_C" :!class /Script/Engine.PrimitiveComponent))
  ;[1 1 1] muestra la animacion de ataque
  (Components|Movement|StopMovementImmediately (Variables|Character|GetCharacterMovement))
  (if (Math|Boolean|ANDBoolean (Variables|Default|GetestaVivo?) (not (Variables|Default|GetestaAtacando?)) true)
    (|PlayAnimationOverridewithCallbacks (Variables|/Script/PaperZD.PaperZDAnimationComponent|GetAnimInstance (Variables|Default|GetAnimationComponent)) "/Game/Ani/CharacterEnemyBaseMeele/AnimSequences/AS_EnemigoAtaqueFinal.AS_EnemigoAtaqueFinal" "AttackEnemigoMeele" 1.0 0.0
      (:then
        (Variables|Default|SetestaAtacando? true)
        (Audio|PlaySound2D "/Game/Sonidos/Espada.Espada" 1.0 1.0 0.0 0 0))
      (:OnCompleted
        (Variables|Default|SetestaAtacando? false)
        (for _array_element _overlappingactors
          (Game|Damage|ApplyDamage _array_element (Math|Conversions|ToFloat(Integer) (* (Variables|Default|Getnivel) 10)) 0 0))
        (if (== (Utilities|Array|Length _overlappingactors) 0)
          (Audio|PlaySound2D "/Game/Sonidos/Espada_viento.Espada_viento" 0.6 _returnvalue 0.0 0 0)
          (else
            (Audio|PlaySound2D "/Game/Sonidos/Player_hurt.Player_hurt" 1.0 _returnvalue 0.0 0 0))))
      (:OnCancelled
        (Variables|Default|SetestaAtacando? false)))))

(fn ConstructionScript
  (|CallParentFunction))

(fn SetDireccionDeColision
  (bind _returnvalue (Transformation|GetVelocity))
  (bind _returnvalue_2 (Transformation|GetActorLocation))
  (bind _box (Variables|Default|GetBox))
  (bind _returnvalue_3 (Class|KismetMathLibrary|VectorNormal2D _returnvalue 0.0001))
  ;[1 1 1] coloca la caja de colision en direccion donde esta mirando
  (if (> (Math|Vector|VectorLength _returnvalue) 0.0)
    (Transformation|SetWorldLocation _box (Math|Vector|MakeVector (+ (.x _returnvalue_2) (* 5e+01 (.x _returnvalue_3))) (+ (.y _returnvalue_2) (* 5e+01 (.y _returnvalue_3))) 2e+01) false false)
    (Transformation|SetWorldRotation _box (Math|Conversions|RotationFromXVector _returnvalue) false false)))

(fn AgarraAlmas
  (return 0.0))

(fn AtaqueDeRango
  (params (posicionHeroe :type Vector :default "0, 0, 0"))
  (return "0, 0, 0"))

(fn PasarStructDatos
  (return ""))

(fn PasarUbicacionHeroe
  (params (ubicacionHeroe :type Vector :default "0, 0, 0"))
  (return))

(fn RecibirUbicacionHeroe
  (return "0, 0, 0"))