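; BP_Character2 is a test player character that handles basic movement through Enhanced Input.
; On BeginPlay it adds the IM_Character mapping context to its player controller's local player subsystem.
; IA_Movimiento feeds its X and Y values into movement input along fixed world axes, independent of camera or actor facing, and prints both values for debugging.
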(event Input|EnhancedActionEvents|EnhancedInputActionIA_Movimiento
  (params (ActionValue :type Vector%202D%20Structure) (ElapsedSeconds :type Float%20%28double-precision%29) (TriggeredSeconds :type Float%20%28double-precision%29) (InputAction :type Input%20Action%20Object%20Reference :default "/Game/BluePrints/Character/Inputs/IA_Movimiento.IA_Movimiento"))
  (Pawn|Input|AddMovementInput "1.000000,0.000000,0.000000" (.x ActionValue) false)
  (Pawn|Input|AddMovementInput "0.000000,1.000000,0.000000" (.y ActionValue) false)
  (Development|PrintString (Utilities|String|Append "Eje en X" (Utilities|String|ToString(Float) (.x ActionValue)) (Utilities|String|ToString(Float) (.y ActionValue)))))

(event EventBeginPlay
  (bind _asplayer_controller (Utilities|Casting|CastToPlayerController (Pawn|GetController)))
  (Input|AddMappingContext (PlayerController|LocalPlayerSubsystems|GetEnhancedInputLocalPlayerSubsystem _asplayer_controller) "/Game/BluePrints/Character/Inputs/IM_Character.IM_Character" 0 "(bIgnoreAllPressedKeysUntilRelease=True,bForceImmediately=False,bNotifyUserSettings=False)"))

(event Collision|EventActorBeginOverlap
  (params (OtherActor :type Actor%20Object%20Reference)))

(event EventTick
  (params (DeltaSeconds :type Float%20%28single-precision%29)))

(fn ConstructionScript)